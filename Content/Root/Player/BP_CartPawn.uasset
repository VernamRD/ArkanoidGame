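; Player paddle ("cart") pawn for a ball-bouncing game that slides via Enhanced Input and spawns an attached ball through BP_GameState to launch.
; Its Geometry Script box mesh and collision rebuild when GameState changes cart width.
; GetNewVelocity fakes a curved paddle by slerping the mirrored velocity sideways by distance from center.
; BeginPlay also runs debug code: traced bounce-vector drawing and a looping timer alternating max FPS between 120 and 20.
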(event Custom|OnCartWidthChanged
  (params (NewWidth :type Float%20%28double-precision%29))
  (CallFunction|SetCartWidth NewWidth))

(event Custom|CustomEvent
  (Utilities|FlowControl|FlipFlop
    (:A
      (Development|ExecuteConsoleCommand "t.MaxFPS 120" 0))
    (:B
      (Development|ExecuteConsoleCommand "t.MaxFPS 20" 0))))

(event Input|EnhancedActionEvents|EnhancedInputActionIA_MoveCart
  (params (ActionValue :type Float%20%28double-precision%29) (ElapsedSeconds :type Float%20%28double-precision%29) (TriggeredSeconds :type Float%20%28double-precision%29) (InputAction :type Input%20Action%20Object%20Reference :default "/Game/Root/Input/IA_MoveCart.IA_MoveCart"))
  (bind _dynamicmesh (Variables|Default|GetDynamicMesh))
  (bind _relativelocation (Variables|/Script/Engine.SceneComponent|GetRelativeLocation _dynamicmesh))
  (bind (_x _y _z) (Math|Vector|BreakVector _relativelocation))
  (Transformation|SetRelativeLocation (Variables|Default|GetDynamicMesh) (Math|Vector|MakeVectorNetQuantize _x (+ _y (* (* (Variables|Settings|GetSensivity) (Math|Float|Absolute(Float) ActionValue)) (Math|Float|Sign(Float) ActionValue))) _z) true false))

(event Input|EnhancedActionEvents|EnhancedInputActionIA_Launch
  (params (ActionValue :type Boolean) (ElapsedSeconds :type Float%20%28double-precision%29) (TriggeredSeconds :type Float%20%28double-precision%29) (InputAction :type Input%20Action%20Object%20Reference :default "/Game/Root/Input/IA_Launch.IA_Launch"))
  (:Started
    (if (CallFunction|IsExistAttachedBalls)
      (CallFunction|LaunchBalls))))

(event EventBeginPlay
  (CallFunction|SpawnBall)
  (bind _asbp_game_state (Utilities|Casting|CastToBP_GameState (Game|GetGameState)))
  (Utilities|FlowControl|Sequence
    (:then_0
      (EventDispatchers|AssignOnCartWidthChanged _asbp_game_state (delegate Custom|OnCartWidthChanged))
      (CallFunction|SetCartWidth (Default|GetCartWidth _asbp_game_state))
      (Debug|DebugDrawBounceVector)
      (Utilities|Time|SetTimerbyEvent (delegate Custom|CustomEvent) 0.5 true))))

(event EventPossessed
  (params (NewController :type Controller%20Object%20Reference))
  (bind _asbp_player_controller (Utilities|Casting|CastToBP_PlayerController NewController))
  (Input|AddMappingContext (PlayerController|LocalPlayerSubsystems|GetEnhancedInputLocalPlayerSubsystem _asbp_player_controller) "/Game/Root/Input/IMC_Game.IMC_Game" 0 "(bIgnoreAllPressedKeysUntilRelease=True,bForceImmediately=False,bNotifyUserSettings=False)"))

(fn ConstructionScript)

(fn SpawnBall
  (bind _ballspawnlocation (Variables|Default|GetBallSpawnLocation))
  (bind _relativelocation (Variables|/Script/Engine.SceneComponent|GetRelativeLocation _ballspawnlocation))
  (bind (_x _y _z) (Math|Vector|BreakVector _relativelocation))
  (bind _asbp_game_state (Utilities|Casting|CastToBP_GameState (Game|GetGameState)))
  (bind _spawnedball (Default|SpawnBall _asbp_game_state (Math|Transform|MakeTransform (Math|Vector|MakeVector _x _y (+ _z (Variables|Default|GetCartHeight)))) self (Math|Vector|GetUpVector (Variables|Default|GetDynamicMesh))))
  (CallFunction|AttachBall _spawnedball))

(fn AttachBall
  (params (Ball :type BP%20Ball%20Object%20Reference))
  (Transformation|AttachComponentToComponent Ball (Variables|Default|GetDynamicMesh) "None" "KeepRelative" "KeepRelative" "KeepRelative" true)
  (Utilities|Array|Add (Variables|Default|GetAttachedBalls) Ball))

(fn IsExistAttachedBalls
  (return (not (Utilities|Array|IsEmpty (Variables|Default|GetAttachedBalls)))))

(fn LaunchBalls
  (for _array_element (Variables|Default|GetAttachedBalls)
    (Transformation|DetachFromActor _array_element "KeepWorld" "KeepRelative" "KeepRelative")
    (Default|Activate _array_element)))

(fn SetCartWidth
  (params (Width :type Float%20%28double-precision%29))
  (bind _cartheight (Variables|Default|GetCartHeight))
  (Variables|Default|SetCartWidth Width)
  (Utilities|FlowControl|Sequence
    (:then_0
      ;[1 1 1] Setup
      (Utilities|FlowControl|DoOnce false
        (:Completed
          (GeometryScript|Scene|SetComponentMaterialList (Variables|Default|GetDynamicMesh) (Utilities|Array|MakeArray (Variables|Default|GetCartMaterial)) 0)
          (bind _returnvalue (DynamicMeshComponent|GetDynamicMesh (Variables|Default|GetDynamicMesh)))
          (Class|GeometryScriptLibraryMeshMaterialFunctions|SetAllTriangleMaterialIDs :TargetMesh _returnvalue :Debug 0))))
    (:then_1
      ;[1 1 1] Generate mesh
      (bind _returnvalue_2 (DynamicMeshComponent|GetDynamicMesh (Variables|Default|GetDynamicMesh)))
      (Utilities|FlowControl|Sequence
        (:then_0
          (DynamicMesh|Reset _returnvalue_2))
        (:then_1
          (Class|GeometryScriptLibraryMeshPrimitiveFunctions|AppendBox :TargetMesh _returnvalue_2 :Transform (Math|Transform|MakeTransform "0, 0, 0") :DimensionX _cartheight :DimensionY (Variables|Default|GetCartWidth) :DimensionZ _cartheight :StepsX 1 :StepsY 1 :StepsZ 1 :Debug 0))))
    (:then_2
      ;[1 1 1] Collision
      (Class|DynamicMeshComponent|UpdateCollision (Variables|Default|GetDynamicMesh) true))))

(fn DebugDrawBounceVector
  (bind _dynamicmesh (Variables|Default|GetDynamicMesh))
  (bind _returnvalue (Transformation|GetWorldLocation _dynamicmesh))
  (bind (_x _y _z) (Math|Vector|BreakVector _returnvalue))
  (for _index (range 0 (Math|Float|Truncate (Variables|Default|GetCartWidth)))
    (bind _outhit (Collision|LineTraceByChannel (+ (Transformation|GetActorLocation) (Math|Vector|MakeVector (+ _index (- _x (/ (Variables|Default|GetCartWidth) 2.0))) _y (+ _z 1e+02))) (Math|Vector|MakeVector (.X (Math|Vector|BreakVector (Math|Vector|MakeVector (+ _index (- _x (/ (Variables|Default|GetCartWidth) 2.0))) _y (+ _z 1e+02)))) (.Y (Math|Vector|BreakVector (Math|Vector|MakeVector (+ _index (- _x (/ (Variables|Default|GetCartWidth) 2.0))) _y (+ _z 1e+02)))) (- (.Z (Math|Vector|BreakVector (Math|Vector|MakeVector (+ _index (- _x (/ (Variables|Default|GetCartWidth) 2.0))) _y (+ _z 1e+02)))) 2e+02)) "TraceTypeQuery3" false (Variables|Default|GetAttachedBalls) "ForDuration" false "(R=1.000000,G=0.000000,B=0.000000,A=1.000000)" "(R=0.000000,G=1.000000,B=0.000000,A=1.000000)" 1e+01))
    (bind _outvelocity (CallFunction|GetNewVelocity (- (Math|Vector|MakeVector (.X (Math|Vector|BreakVector (Math|Vector|MakeVector (+ _index (- _x (/ (Variables|Default|GetCartWidth) 2.0))) _y (+ _z 1e+02)))) (.Y (Math|Vector|BreakVector (Math|Vector|MakeVector (+ _index (- _x (/ (Variables|Default|GetCartWidth) 2.0))) _y (+ _z 1e+02)))) (- (.Z (Math|Vector|BreakVector (Math|Vector|MakeVector (+ _index (- _x (/ (Variables|Default|GetCartWidth) 2.0))) _y (+ _z 1e+02)))) 2e+02)) (+ (Transformation|GetActorLocation) (Math|Vector|MakeVector (+ _index (- _x (/ (Variables|Default|GetCartWidth) 2.0))) _y (+ _z 1e+02)))) (.ImpactPoint (Collision|BreakHitResult _outhit)) (.ImpactNormal (Collision|BreakHitResult _outhit))))
    (Collision|LineTraceByChannel (.ImpactPoint (Collision|BreakHitResult _outhit)) (+ (.ImpactPoint (Collision|BreakHitResult _outhit)) _outvelocity) "TraceTypeQuery3" false (Variables|Default|GetAttachedBalls) "ForDuration" false "(R=0.000000,G=1.000000,B=0.966424,A=1.000000)" "(R=0.000000,G=1.000000,B=0.976368,A=1.000000)" 1e+01)))

(fn GetNewVelocity
  (params (InputVelocty :type Vector :default "0, 0, 0") (ImpactPoint :type Vector :default "0, 0, 0") (ImpactNormal :type Vector :default "0, 0, 0"))
  (bind (_x _y _z) (Math|Vector|BreakVector ImpactPoint))
  (bind _dynamicmesh (Variables|Default|GetDynamicMesh))
  (bind _dynamicmesh_2 (Variables|Default|GetDynamicMesh))
  (bind _dynamicmesh_3 (Variables|Default|GetDynamicMesh))
  (bind _cartwidth (Variables|Default|GetCartWidth))
  (bind _returnvalue (Math|Vector|GetRightVector _dynamicmesh_3))
  (bind _returnvalue_2 (Transformation|GetWorldLocation _dynamicmesh_2))
  (bind _returnvalue_3 (- ImpactPoint _returnvalue_2))
  (return (* (Class|KismetMathLibrary|VectorSlerpNormals (Math|Vector|Normalize (Math|Vector|MirrorVectorbyNormal InputVelocty ImpactNormal)) (Math|Vector|Normalize (Math|Vector|SelectVector (Math|Vector|NegateVector _returnvalue) _returnvalue (> (Math|Vector|Distance(Vector) _returnvalue_3 (* (Math|Vector|GetRightVector _dynamicmesh) _cartwidth)) (Math|Vector|Distance(Vector) _returnvalue_3 (* _cartwidth (Math|Vector|NegateVector (Math|Vector|GetRightVector _dynamicmesh))))))) (/ (* (Variables|Settings|GetCartSphereBounceModifier) (Math|Vector|Distance(Vector) (Math|Vector|MakeVector _x _y (- _z (Variables|Default|GetCartHeight))) (Transformation|GetWorldLocation (Variables|Default|GetDynamicMesh)))) (/ (Variables|Default|GetCartWidth) 2.0))) (Math|Vector|VectorLength InputVelocty))))