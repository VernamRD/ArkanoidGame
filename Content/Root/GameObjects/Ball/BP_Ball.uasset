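; Bouncing ball actor that, once activated, moves by sphere-tracing its path each tick instead of using physics.
; On impact, BPI_BallVelocityChanger actors supply a new velocity; others mirror it, with BPI_BallHitable ones notified first, and the trace recurses.
; Size and speed follow GameState events, with size rebuilding the dynamic-mesh sphere and collision radius.
; Overlaps with owned actors push the ball out through a recursive search for free space.
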(event OnComponentBeginOverlap(Sphere)
  (params (OverlappedComponent :type Primitive%20Component%20Object%20Reference) (OtherActor :type Actor%20Object%20Reference) (OtherComp :type Primitive%20Component%20Object%20Reference) (OtherBodyIndex :type Integer) (bFromSweep :type Boolean) (SweepResult :type Hit%20Result%20Structure%20%28by%20ref%29))
  ;[0.2552 0.2552 0.2552 1 40] Extraction the ball if it is inside a collision
  (Utilities|IsValid (Components|GetOwner OtherActor)
    (:Is%20Valid
      (Variables|Default|SetVelocityVector (Math|Vector|Normalize (- (Transformation|GetActorLocation) (Transformation|GetWorldLocation OtherComp))))
      (bind _newlocation (CallFunction|FindAvailableLocationAlongVelocity 1.0))
      (Transformation|SetActorLocation _newlocation false false))))

(event Custom|OnBallSizeChanged
  (params (NewBallSize :type Float%20%28double-precision%29))
  (CallFunction|SetupBall NewBallSize))

(event Custom|OnBallVelocityChanged_Event
  (params (NewVelocity :type Float%20%28double-precision%29))
  (Variables|Default|SetBallVelocity NewVelocity))

(event EventBeginPlay
  (Utilities|FlowControl|Sequence
    (:then_0
      (bind _asbp_game_state (Utilities|Casting|CastToBP_GameState (Game|GetGameState)))
      (EventDispatchers|AssignOnBallSizeChanged _asbp_game_state (delegate Custom|OnBallSizeChanged))
      (CallFunction|OnBallSizeChanged (Default|GetBallSize _asbp_game_state))
      (EventDispatchers|AssignOnBallVelocityChanged _asbp_game_state (delegate Custom|OnBallVelocityChanged_Event))
      (CallFunction|OnBallVelocityChangedEvent (Default|GetBallVelocity _asbp_game_state)))
    (:then_1
      (Variables|Default|SetVelocityVector (Math|Vector|Normalize (Variables|Default|GetVelocityVector))))))

(event Collision|EventActorBeginOverlap
  (params (OtherActor :type Actor%20Object%20Reference)))

(event EventTick
  (params (DeltaSeconds :type Float%20%28single-precision%29))
  (if (Variables|Default|GetbActivated)
    (CallFunction|Trace (* DeltaSeconds (Variables|Default|GetVelocityVector) (Variables|Default|GetBallVelocity)))))

(fn ConstructionScript)

(fn Activate
  (Variables|Default|SetbActivated true))

(fn Trace
  (params (VectorResultVelocity :type Vector))
  (bind _outhit (Collision|SphereTraceByChannel (Transformation|GetActorLocation) (+ VectorResultVelocity (Transformation|GetActorLocation)) (Variables|Default|GetBallSize) "TraceTypeQuery3" false 0 "None"))
  (if (.bBlockingHit (Collision|BreakHitResult _outhit))
    (LocalVariables|SetDistance (.Distance (Collision|BreakHitResult _outhit)))
    (LocalVariables|SetImpactPoint (.ImpactPoint (Collision|BreakHitResult _outhit)))
    (LocalVariables|SetImpactNormal (.ImpactNormal (Collision|BreakHitResult _outhit)))
    (if (Utilities|DoesObjectImplementInterface (.HitActor (Collision|BreakHitResult _outhit)) "/Game/Root/GameObjects/Ball/BPI_BallVelocityChanger.BPI_BallVelocityChanger_C")
      ;[0.2708 0.2708 0.2708 1 40] Cart hit
      (bind _outvelocity (Class|BPIBallVelocityChanger|GetNewVelocity(Message) (.HitActor (Collision|BreakHitResult _outhit)) VectorResultVelocity (LocalVariables|GetImpactPoint) (LocalVariables|GetImpactNormal)))
      (Variables|Default|SetVelocityVector (Math|Vector|Normalize _outvelocity))
      (CallFunction|Trace (* _outvelocity (/ (LocalVariables|GetDistance) (Math|Vector|VectorLength VectorResultVelocity))))
      (elif (Utilities|DoesObjectImplementInterface (.HitActor (Collision|BreakHitResult _outhit)) "/Game/Root/GameObjects/Ball/BPI_BallHitable.BPI_BallHitable_C")
        (Utilities|FlowControl|Sequence
          (:then_0
            (Class|BPIBallHitable|Hit(Message) (.HitActor (Collision|BreakHitResult _outhit)) self (LocalVariables|GetImpactPoint)))
          (:then_1
            ;[0.2708 0.2708 0.2708 1 40] Default mirror velocity
            (Variables|Default|SetVelocityVector (Math|Vector|Normalize (Math|Vector|MirrorVectorbyNormal VectorResultVelocity (LocalVariables|GetImpactNormal))) :!label _label)
            (CallFunction|Trace (* (Math|Vector|MirrorVectorbyNormal VectorResultVelocity (LocalVariables|GetImpactNormal)) (/ (LocalVariables|GetDistance) (Math|Vector|VectorLength VectorResultVelocity))))))
        (else
          (goto _label))))
    (else
      (Transformation|SetActorLocation (.TraceEnd (Collision|BreakHitResult _outhit)) true false))))

(fn SetupBall
  (params (InBallSize :type Float%20%28double-precision%29))
  (Variables|Default|SetBallSize InBallSize)
  (GeometryScript|Scene|SetComponentMaterialList (Variables|Default|GetDynamicMesh) (Utilities|Array|MakeArray (Variables|Default|GetMaterial)) 0)
  (bind _returnvalue (DynamicMeshComponent|GetDynamicMesh (Variables|Default|GetDynamicMesh)))
  (bind _returnvalue_2 (DynamicMesh|Reset _returnvalue))
  (Class|GeometryScriptLibraryMeshPrimitiveFunctions|AppendSphereBox :TargetMesh _returnvalue_2 :Transform (Math|Transform|MakeTransform (Variables|/Script/Engine.SceneComponent|GetRelativeLocation (Variables|Default|GetDynamicMesh))) :Radius (Variables|Default|GetBallSize) :Debug 0)
  (Components|Sphere|SetSphereRadius (Variables|Default|GetSphere) (Variables|Default|GetBallSize) true))

(fn FindAvailableLocationAlongVelocity
  (params (Distance :type Float%20%28double-precision%29))
  (bind _output_get (LocalVariables|SetTestLocation (+ (* (Variables|Default|GetVelocityVector) Distance) (Transformation|GetActorLocation))))
  (bind _outhit (Collision|SphereTraceByChannel _output_get _output_get (Variables|Default|GetBallSize) "TraceTypeQuery3" false 0 "None"))
  (if (.bBlockingHit (Collision|BreakHitResult _outhit))
    (bind _newlocation (CallFunction|FindAvailableLocationAlongVelocity (+ Distance 1.0)))
    (return _newlocation)
    (else
      (return (LocalVariables|GetTestLocation)))))