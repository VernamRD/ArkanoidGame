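; BP_Block is a destructible block that loses one HP per hit and asks the game state to destroy it at zero.
; On BeginPlay it caches BP_GameState, builds a rectangle with Geometry Script on a dynamic mesh component, and fits its collision box to the game state's block size.
; A dynamic material instance recolors the block to the game state's color for its remaining HP.
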(event EventBeginPlay
  (Utilities|FlowControl|Sequence
    (:then_0
      (bind _asbp_game_state (Utilities|Casting|CastToBP_GameState (Game|GetGameState)))
      (Variables|Default|SetGameState _asbp_game_state))
    (:then_1
      (CallFunction|SetupBlockMesh))
    (:then_2
      (Variables|Default|SetHP (Variables|Default|GetMaxHP))
      (CallFunction|OnHPUpdate))))

(event Collision|EventActorBeginOverlap
  (params (OtherActor :type Actor%20Object%20Reference)))

(event EventTick
  (params (DeltaSeconds :type Float%20%28single-precision%29)))

(event EventHit
  (params (Ball :type BP%20Ball%20Object%20Reference) (ImpactPoint :type Vector :default "0, 0, 0"))
  (CallFunction|DecreaseHP))

(fn ConstructionScript)

(fn DecreaseHP
  (bind _result (Math|Integer|DecrementInt (Variables|Default|GetHP))
    (:%20%20
      (if (<= _result 0)
        (Default|DestroyBlock (Variables|Default|GetGameState) self)
        (else
          (CallFunction|OnHPUpdate))))))

(fn SetupBlockMesh
  (bind _dynamicmesh (Variables|Default|GetDynamicMesh))
  (bind _gamestate (Variables|Default|GetGameState))
  (bind _default_block_height (Default|GetBlockHeight _gamestate))
  (bind _default_block_width (Default|GetBlockWidth _gamestate))
  (bind _returnvalue (Rendering|Material|CreateDynamicMaterialInstance (Variables|Default|GetMaterial) "None" "Transient" :!class /Script/Engine.KismetMaterialLibrary))
  (bind _output_get (Variables|Default|SetDynamicMateriaInstance _returnvalue))
  (GeometryScript|Scene|SetComponentMaterialList _dynamicmesh (Utilities|Array|MakeArray _output_get) 0)
  (bind _returnvalue_2 (DynamicMeshComponent|GetDynamicMesh _dynamicmesh))
  (bind _returnvalue_3 (DynamicMesh|Reset _returnvalue_2))
  (Class|GeometryScriptLibraryMeshPrimitiveFunctions|AppendRectangleXY :TargetMesh _returnvalue_3 :Transform (Math|Transform|MakeTransform "0, 0, 0") :DimensionX _default_block_width :DimensionY _default_block_height :Debug 0)
  (Components|Box|SetBoxExtent (Variables|Default|GetBox) (Math|Vector|MakeVector (/ _default_block_width 2.0) (/ _default_block_height 2.0) 1e+02) true))

(fn OnHPUpdate
  (Rendering|Material|SetVectorParameterValue (Variables|Default|GetDynamicMateriaInstance) "Color" (Default|GetColorPerBlockHP (Variables|Default|GetGameState) (Variables|Default|GetHP)) :!class /Script/Engine.MaterialInstanceDynamic))