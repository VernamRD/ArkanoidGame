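; Level generator actor that builds the boundary of a play area from Width and Height, including a game-over bound at the bottom.
; The construction script positions and resizes four box bounds, then uses Geometry Script to append matching rectangles to a reset DynamicMesh with the unbreakable material.
; DebugVisibility toggles whether the boxes show in game.
; The event graph has no logic.
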(event EventBeginPlay)

(event Collision|EventActorBeginOverlap
  (params (OtherActor :type Actor%20Object%20Reference)))

(event EventTick
  (params (DeltaSeconds :type Float%20%28single-precision%29)))

(fn ConstructionScript
  (Setup|SetupBound)
  (CallFunction|DebugDrawCollisions))

(fn DebugDrawCollisions
  (bind _bdebugvisibility (Variables|Default|GetbDebugVisibility))
  (bind _returnvalue (not _bdebugvisibility))
  (Utilities|FlowControl|Sequence
    (:then_0
      (Development|SetHiddeninGame (Variables|Default|GetLeftBound) _returnvalue false))
    (:then_1
      (Development|SetHiddeninGame (Variables|Default|GetRightBound) _returnvalue false))
    (:then_2
      (Development|SetHiddeninGame (Variables|Default|GetTopBound) _returnvalue false))
    (:then_3
      (Development|SetHiddeninGame (Variables|Default|GetGameOverBound) _returnvalue false))))

(fn SetupBound
  (bind _dynamicmesh (Variables|Default|GetDynamicMesh))
  (bind _returnvalue (DynamicMeshComponent|GetDynamicMesh _dynamicmesh))
  (bind _returnvalue_2 (DynamicMesh|Reset _returnvalue))
  (Class|GeometryScriptLibraryMeshMaterialFunctions|SetAllTriangleMaterialIDs :TargetMesh _returnvalue_2 :Debug 0)
  (GeometryScript|Scene|SetComponentMaterialList _dynamicmesh (Utilities|Array|MakeArray "/Game/Root/Materials/MI_Unbreakable.MI_Unbreakable") 0)
  (Utilities|FlowControl|Sequence
    (:then_0
      (Setup|SetupVerticalBound (Variables|Default|GetLeftBound) (* (CallFunction|GetHorizontalBoundPosition) -1.0)))
    (:then_1
      (Setup|SetupVerticalBound (Variables|Default|GetRightBound) (CallFunction|GetHorizontalBoundPosition)))
    (:then_2
      (Setup|SetupHorizontalBound (Variables|Default|GetTopBound) (CallFunction|GetVerticalBoundPosition)))
    (:then_3
      (Setup|SetupHorizontalBound (Variables|Default|GetGameOverBound) (* (CallFunction|GetVerticalBoundPosition) -1.0)))))

(fn SetupVerticalBound
  (params (Bound :type Box%20Component%20Object%20Reference) (NewLocation_X :type Float%20%28double-precision%29))
  (bind _boxextent (Variables|/Script/Engine.BoxComponent|GetBoxExtent Bound))
  (bind _boxextent_2 (Variables|/Script/Engine.BoxComponent|GetBoxExtent Bound))
  (bind _returnvalue (* _boxextent_2 2.0))
  (bind (_x _y _z) (Math|Vector|BreakVector _returnvalue))
  (Transformation|SetRelativeLocation Bound (Math|Vector|MakeVector NewLocation_X 0.0 0.0) false true)
  (Components|Box|SetBoxExtent Bound (Math|Vector|MakeVector (.x _boxextent) (.y _boxextent) (/ (Variables|Default|GetHeight) 2.0)) false)
  (bind _returnvalue_2 (DynamicMeshComponent|GetDynamicMesh (Variables|Default|GetDynamicMesh)))
  (Class|GeometryScriptLibraryMeshPrimitiveFunctions|AppendRectangleXY :TargetMesh _returnvalue_2 :Transform (Math|Transform|MakeTransform (Math|Vector|MakeVector NewLocation_X 0.0 0.0) "0.000000,0.000000,90.000000") :DimensionX _x :DimensionY _z :Debug 0))

(fn GetHorizontalBoundPosition
  (return (+ (/ (Variables|Default|GetWidth) 2.0) (Variables|Default|GetDefaultBoxBoundSize))))

(fn SetupHorizontalBound
  (params (Bound :type Box%20Component%20Object%20Reference) (NewLocation_Z :type Float%20%28double-precision%29))
  (bind _boxextent (Variables|/Script/Engine.BoxComponent|GetBoxExtent Bound))
  (bind _boxextent_2 (Variables|/Script/Engine.BoxComponent|GetBoxExtent Bound))
  (bind _returnvalue (* _boxextent_2 2.0))
  (bind (_x _y _z) (Math|Vector|BreakVector _returnvalue))
  (Transformation|SetRelativeLocation Bound (Math|Vector|MakeVector 0.0 0.0 NewLocation_Z) false true)
  (Components|Box|SetBoxExtent Bound (Math|Vector|MakeVector (+ (/ (Variables|Default|GetWidth) 2.0) (* (Variables|Default|GetDefaultBoxBoundSize) 2.0)) (.y _boxextent) (.z _boxextent)) false)
  (bind _returnvalue_2 (DynamicMeshComponent|GetDynamicMesh (Variables|Default|GetDynamicMesh)))
  (Class|GeometryScriptLibraryMeshPrimitiveFunctions|AppendRectangleXY :TargetMesh _returnvalue_2 :Transform (Math|Transform|MakeTransform (Math|Vector|MakeVector 0.0 0.0 NewLocation_Z) "0.000000,0.000000,90.000000") :DimensionX _x :DimensionY _z :Debug 0))

(fn GetVerticalBoundPosition
  (return (+ (/ (Variables|Default|GetHeight) 2.0) (Variables|Default|GetDefaultBoxBoundSize))))