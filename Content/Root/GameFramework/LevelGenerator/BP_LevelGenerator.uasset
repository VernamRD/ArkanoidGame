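; BP_LevelGenerator builds the brick-breaker arena and spawns each level's blocks.
; SetupBound sizes box bounds and draws left, right and top walls with Geometry Script, both in construction and at BeginPlay.
; GameState triggers async loading of a DataTable whose rows of HP values become the block grid, and is told when all are destroyed.
; The bottom bound removes balls and power-ups, and DamageAllBlock damages every block.
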(event OnComponentBeginOverlap(GameOverBound)
  (params (OverlappedComponent :type Primitive%20Component%20Object%20Reference) (OtherActor :type Actor%20Object%20Reference) (OtherComp :type Primitive%20Component%20Object%20Reference) (OtherBodyIndex :type Integer) (bFromSweep :type Boolean) (SweepResult :type Hit%20Result%20Structure%20%28by%20ref%29))
  (bind _returnvalue (Utilities|GetClass OtherActor))
  (if (Utilities|ClassIsChildOf _returnvalue "/Game/Root/GameFramework/GameObjects/Ball/BP_Ball.BP_Ball_C")
    (Default|DestroyBall (Variables|Default|GetGameState) (.AsBP%20Ball (Utilities|Casting|CastToBP_Ball OtherActor)))
    (elif (Utilities|ClassIsChildOf _returnvalue "/Game/Root/GameFramework/GameObjects/PowerUp/BP_PowerUPBase.BP_PowerUPBase_C")
      (Actor|DestroyActor OtherActor))))

(event Custom|TryGenerateLevel
  (params (LevelIndex :type Integer))
  (bind _object (Utilities|AsyncLoadAsset (Default|GetLevelData (Variables|Default|GetGameState)))
    (:Completed
      (bind _asdata_table (Utilities|Casting|CastToDataTable _object))
      (CallFunction|GenerateLevel _asdata_table))))

(event EventBeginPlay
  (Utilities|FlowControl|Sequence
    (:then_0
      (bind _asbp_game_state (Utilities|Casting|CastToBP_GameState (Game|GetGameState)))
      (bind _output_get (Variables|Default|SetGameState _asbp_game_state))
      (Variables|Default|SetWidth (Default|GetAreaWidth _output_get)))
    (:then_1
      (Setup|SetupBound))
    (:then_2
      (EventDispatchers|AssignOnStartNewLevel (Variables|Default|GetGameState) (delegate Custom|TryGenerateLevel))
      (Default|StartNewLevel (Variables|Default|GetGameState)))))

(event Collision|EventActorBeginOverlap
  (params (OtherActor :type Actor%20Object%20Reference)))

(event EventTick
  (params (DeltaSeconds :type Float%20%28single-precision%29)))

(fn ConstructionScript
  (Setup|SetupBound)
  (CallFunction|DebugDrawCollisions))

(fn DebugDrawCollisions
  (bind _bdebugvisibility (Variables|Default|GetbDebugVisibility))
  (bind _returnvalue (not _bdebugvisibility))
  (Utilities|FlowControl|Sequence
    (:then_0
      (Development|SetHiddeninGame (Variables|Default|GetLeftBound) _returnvalue false))
    (:then_1
      (Development|SetHiddeninGame (Variables|Default|GetRightBound) _returnvalue false))
    (:then_2
      (Development|SetHiddeninGame (Variables|Default|GetTopBound) _returnvalue false))
    (:then_3
      (Development|SetHiddeninGame (Variables|Default|GetGameOverBound) _returnvalue false))))

(fn SetupBound
  (bind _dynamicmesh (Variables|Default|GetDynamicMesh))
  (bind _returnvalue (DynamicMeshComponent|GetDynamicMesh _dynamicmesh))
  (DynamicMesh|Reset _returnvalue)
  (GeometryScript|Scene|SetComponentMaterialList _dynamicmesh (Utilities|Array|MakeArray "/Game/Root/Materials/MI_Unbreakable.MI_Unbreakable") 0)
  (Utilities|FlowControl|Sequence
    (:then_0
      (Setup|SetupVerticalBound (Variables|Default|GetLeftBound) (* (CallFunction|GetHorizontalBoundPosition) -1.0)))
    (:then_1
      (Setup|SetupVerticalBound (Variables|Default|GetRightBound) (CallFunction|GetHorizontalBoundPosition)))
    (:then_2
      (Setup|SetupHorizontalBound (Variables|Default|GetTopBound) (CallFunction|GetVerticalBoundPosition) true))
    (:then_3
      (Setup|SetupHorizontalBound (Variables|Default|GetGameOverBound) (* (CallFunction|GetVerticalBoundPosition) -1.0) false))))

(fn SetupVerticalBound
  (params (Bound :type Box%20Component%20Object%20Reference) (NewLocation_X :type Float%20%28double-precision%29))
  (bind _boxextent (Variables|/Script/Engine.BoxComponent|GetBoxExtent Bound))
  (bind _boxextent_2 (Variables|/Script/Engine.BoxComponent|GetBoxExtent Bound))
  (bind _returnvalue (* _boxextent_2 2.0))
  (bind (_x _y _z) (Math|Vector|BreakVector _returnvalue))
  (Transformation|SetRelativeLocation Bound (Math|Vector|MakeVector NewLocation_X 0.0 0.0) false true)
  (Components|Box|SetBoxExtent Bound (Math|Vector|MakeVector (.x _boxextent) (.y _boxextent) (/ (Variables|Default|GetHeight) 2.0)) false)
  (bind _returnvalue_2 (DynamicMeshComponent|GetDynamicMesh (Variables|Default|GetDynamicMesh)))
  (Class|GeometryScriptLibraryMeshPrimitiveFunctions|AppendRectangleXY :TargetMesh _returnvalue_2 :Transform (Math|Transform|MakeTransform (Math|Vector|MakeVector NewLocation_X 0.0 0.0) "0.000000,0.000000,90.000000") :DimensionX _x :DimensionY _z :Debug 0))

(fn GetHorizontalBoundPosition
  (return (+ (/ (Variables|Default|GetWidth) 2.0) (Variables|Default|GetDefaultBoxBoundSize))))

(fn SetupHorizontalBound
  (params (Bound :type Box%20Component%20Object%20Reference) (NewLocation_Z :type Float%20%28double-precision%29) (bCreateMesh :type Boolean))
  (bind _boxextent (Variables|/Script/Engine.BoxComponent|GetBoxExtent Bound))
  (bind _boxextent_2 (Variables|/Script/Engine.BoxComponent|GetBoxExtent Bound))
  (bind _returnvalue (* _boxextent_2 2.0))
  (bind (_x _y _z) (Math|Vector|BreakVector _returnvalue))
  (Transformation|SetRelativeLocation Bound (Math|Vector|MakeVector 0.0 0.0 NewLocation_Z) false true)
  (Components|Box|SetBoxExtent Bound (Math|Vector|MakeVector (+ (/ (Variables|Default|GetWidth) 2.0) (* (Variables|Default|GetDefaultBoxBoundSize) 2.0)) (.y _boxextent) (.z _boxextent)) false)
  (if bCreateMesh
    (bind _returnvalue_2 (DynamicMeshComponent|GetDynamicMesh (Variables|Default|GetDynamicMesh)))
    (Class|GeometryScriptLibraryMeshPrimitiveFunctions|AppendRectangleXY :TargetMesh _returnvalue_2 :Transform (Math|Transform|MakeTransform (Math|Vector|MakeVector 0.0 0.0 NewLocation_Z) "0.000000,0.000000,90.000000") :DimensionX _x :DimensionY _z :Debug 0)))

(fn GetVerticalBoundPosition
  (return (+ (/ (Variables|Default|GetHeight) 2.0) (Variables|Default|GetDefaultBoxBoundSize))))

(fn GenerateLevel
  (params (LevelData :type Data%20Table%20Object%20Reference))
  (bind _gamestate (Variables|Default|GetGameState))
  (LocalVariables|SetCachedBlockWidth (Default|GetBlockWidth _gamestate))
  (LocalVariables|SetCachedBlockHeight (Default|GetBlockHeight _gamestate))
  (bind _outrownames (DataTable|GetDataTableRowNames LevelData))
  (for (_array_element _array_index) _outrownames
    (bind _returnvalue (Utilities|GetDataTableRow LevelData _array_element)
      (:then
        (for (_array_element_2 _array_index_2) (Utilities|Struct|BreakF_Block _returnvalue)
          (if (> _array_element_2 0)
            (bind _returnvalue_2 (Game|SpawnActorfromClass "/Game/Root/GameFramework/GameObjects/Blocks/BP_Block.BP_Block_C" (Math|Transform|MakeTransform (+ (Math|Vector|MakeVector (* (* _array_index_2 (LocalVariables|GetCachedBlockWidth)) -1.0) 0.0 (* (* _array_index (LocalVariables|GetCachedBlockHeight)) -1.0)) (Transformation|GetWorldLocation (Variables|Default|GetBlocksOrigin)))) "Undefined" "MultiplyWithRoot" 0 _array_element_2 0))
            (Transformation|AttachComponentToComponent _returnvalue_2 (Variables|Default|GetBlocksOrigin) "None" "KeepWorld" "KeepWorld" "KeepWorld" true)
            (Utilities|Array|Add (Variables|Default|GetBlocks) _returnvalue_2)
            (EventDispatchers|BindEventtoOnBlockDestroyed _returnvalue_2 (EventDispatchers|CreateEvent :!event OnBlockDestroyed))))))))

(fn OnBlockDestroyed
  (params (Block :type BP%20Block%20Object%20Reference))
  (Default|OnDestroyBlock (Variables|Default|GetGameState) Block)
  (Utilities|Array|RemoveItem (Variables|Default|GetBlocks) Block)
  (if (Utilities|Array|IsEmpty (Variables|Default|GetBlocks))
    (Default|FinishLevel (Variables|Default|GetGameState))))

(fn DamageAllBlock
  (bind _output_get (LocalVariables|SetCachedBlocks (Variables|Default|GetBlocks)))
  (for _array_element _output_get
    (Default|DecreaseHP _array_element)))