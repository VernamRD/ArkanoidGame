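; BP_Ball is a bouncing ball that moves each tick once activated, taking its size and speed from BP_GameState delegates.
; Size changes rebuild a Geometry Script sphere mesh and resize the collision sphere.
; Movement uses recursive sphere traces: hits deflect the direction through BPI_BallVelocityChanger or mirror it by the normal.
; Each retrace starts from the unchanged location, scaled by hit-distance fraction, until a clear trace moves the actor.
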(event Custom|OnBallSizeChanged
  (params (NewBallSize :type Float%20%28double-precision%29))
  (CallFunction|SetupBall NewBallSize))

(event Custom|OnBallVelocityChanged_Event
  (params (NewVelocity :type Float%20%28double-precision%29))
  (Variables|Default|SetBallVelocity NewVelocity))

(event EventBeginPlay
  (Utilities|FlowControl|Sequence
    (:then_0
      (bind _asbp_game_state (Utilities|Casting|CastToBP_GameState (Game|GetGameState)))
      (EventDispatchers|AssignOnBallSizeChanged _asbp_game_state (delegate Custom|OnBallSizeChanged))
      (CallFunction|OnBallSizeChanged (Default|GetBallSize _asbp_game_state))
      (EventDispatchers|AssignOnBallVelocityChanged _asbp_game_state (delegate Custom|OnBallVelocityChanged_Event))
      (CallFunction|OnBallVelocityChangedEvent (Default|GetBallVelocity _asbp_game_state)))
    (:then_1
      (Variables|Default|SetVelocityVector (Math|Vector|Normalize (Variables|Default|GetVelocityVector))))))

(event Collision|EventActorBeginOverlap
  (params (OtherActor :type Actor%20Object%20Reference)))

(event EventTick
  (params (DeltaSeconds :type Float%20%28single-precision%29))
  (if (Variables|Default|GetbActivated)
    (CallFunction|Trace (* DeltaSeconds (Variables|Default|GetVelocityVector) (Variables|Default|GetBallVelocity)))))

(fn ConstructionScript)

(fn Activate
  (Variables|Default|SetbActivated true))

(fn Trace
  (params (VectorResultVelocity :type Vector))
  (bind _outhit (Collision|SphereTraceByChannel (Transformation|GetActorLocation) (+ VectorResultVelocity (Transformation|GetActorLocation)) (Variables|Default|GetBallSize) "TraceTypeQuery3" false 0 "None"))
  (if (.bBlockingHit (Collision|BreakHitResult _outhit))
    (if (Utilities|DoesObjectImplementInterface (.HitActor (Collision|BreakHitResult _outhit)) "/Game/Root/Player/BPI_BallVelocityChanger.BPI_BallVelocityChanger_C")
      ;[0.2708 0.2708 0.2708 1 40] Cart hit
      (bind _outvelocity (Class|BPIBallVelocityChanger|GetNewVelocity(Message) (.HitActor (Collision|BreakHitResult _outhit)) VectorResultVelocity (.ImpactPoint (Collision|BreakHitResult _outhit)) (.ImpactNormal (Collision|BreakHitResult _outhit))))
      (Variables|Default|SetVelocityVector (Math|Vector|Normalize _outvelocity))
      (CallFunction|Trace (* _outvelocity (/ (.Distance (Collision|BreakHitResult _outhit)) (Math|Vector|VectorLength VectorResultVelocity))))
      (else
        ;[0.2708 0.2708 0.2708 1 40] Default mirror velocity
        (Variables|Default|SetVelocityVector (Math|Vector|Normalize (Math|Vector|MirrorVectorbyNormal VectorResultVelocity (.ImpactNormal (Collision|BreakHitResult _outhit)))))
        (CallFunction|Trace (* (Math|Vector|MirrorVectorbyNormal VectorResultVelocity (.ImpactNormal (Collision|BreakHitResult _outhit))) (/ (.Distance (Collision|BreakHitResult _outhit)) (Math|Vector|VectorLength VectorResultVelocity))))))
    (else
      (Transformation|SetActorLocation (.TraceEnd (Collision|BreakHitResult _outhit)) true false))))

(fn SetupBall
  (params (InBallSize :type Float%20%28double-precision%29))
  (Variables|Default|SetBallSize InBallSize)
  (GeometryScript|Scene|SetComponentMaterialList (Variables|Default|GetDynamicMesh) (Utilities|Array|MakeArray (Variables|Default|GetMaterial)) 0)
  (bind _returnvalue (DynamicMeshComponent|GetDynamicMesh (Variables|Default|GetDynamicMesh)))
  (bind _returnvalue_2 (DynamicMesh|Reset _returnvalue))
  (bind _returnvalue_3 (Class|GeometryScriptLibraryMeshMaterialFunctions|SetAllTriangleMaterialIDs :TargetMesh _returnvalue_2 :Debug 0))
  (Class|GeometryScriptLibraryMeshPrimitiveFunctions|AppendSphereBox :TargetMesh _returnvalue_3 :Transform (Math|Transform|MakeTransform (Variables|/Script/Engine.SceneComponent|GetRelativeLocation (Variables|Default|GetDynamicMesh))) :Radius (Variables|Default|GetBallSize) :Debug 0)
  (Components|Sphere|SetSphereRadius (Variables|Default|GetSphere) (Variables|Default|GetBallSize) true))