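; Game state for a Breakout-style game, holding score, remaining balls, active balls, level progress and cart and ball stats.
; Defaults, levels, scoring and power-up drop chances come from a settings asset, and event dispatchers broadcast changes.
; Power-ups adjust stats within clamped multiples of defaults, add lives, or spawn two extra balls without spending any.
; Losing the last active ball requests a respawn or ends the game; destroyed blocks award score and may drop power-ups.
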(event EventBeginPlay
  (bind _settingsasset (Variables|Default|GetSettingsAsset))
  (Utilities|FlowControl|Sequence
    (:then_0
      (bind _output_get (Variables|DefaultValues|SetDefaultCartWidth (Variables|/Script/Arkanoid.ArkanoidGameSettingsAsset|GetDefaultCartWidth _settingsasset)))
      (Game|SetCartWidth _output_get))
    (:then_1
      (bind _output_get_2 (Variables|DefaultValues|SetDefaultBallSize (Variables|/Script/Arkanoid.ArkanoidGameSettingsAsset|GetDefaultBallSize _settingsasset)))
      (Game|SetBallSize _output_get_2))
    (:then_2
      (bind _output_get_3 (Variables|DefaultValues|SetDefaultBallSpeed (Variables|/Script/Arkanoid.ArkanoidGameSettingsAsset|GetDefaultBallVelocity _settingsasset)))
      (Game|SetBallSpeed _output_get_3))
    (:then_3
      (bind _output_get_4 (Variables|Default|SetBallsRemaining (Variables|/Script/Arkanoid.ArkanoidGameSettingsAsset|GetBallsCount _settingsasset)))
      (Default|CallOnBallsRemainingChanged _output_get_4))
    (:then_4
      (Variables|Default|SetbReady true)
      (Default|CallOnReady))))

(fn ConstructionScript)

(fn IsAllowSpawnBall
  (return (> (Variables|Default|GetBallsRemaining) 0)))

(fn SetCartWidth
  (params (CartWidth :type Float%20%28double-precision%29))
  (bind _defaultcartwidth (Variables|DefaultValues|GetDefaultCartWidth))
  (bind _maxmodifierfromdefaultvalue (Variables|Static|GetMaxModifierFromDefaultValue))
  (bind _output_get (Variables|Default|SetCurrentCartWidth (Math|Float|Clamp(Float) CartWidth (/ _defaultcartwidth _maxmodifierfromdefaultvalue) (* _defaultcartwidth _maxmodifierfromdefaultvalue))))
  (Default|CallOnCartWidthChanged _output_get))

(fn SetBallSize
  (params (BallSize :type Float%20%28double-precision%29))
  (bind _defaultballsize (Variables|DefaultValues|GetDefaultBallSize))
  (bind _maxmodifierfromdefaultvalue (Variables|Static|GetMaxModifierFromDefaultValue))
  (bind _output_get (Variables|Default|SetCurrentBallSize (Math|Float|Clamp(Float) BallSize (/ _defaultballsize _maxmodifierfromdefaultvalue) (* _defaultballsize _maxmodifierfromdefaultvalue))))
  (Default|CallOnBallSizeChanged _output_get))

(fn SetBallSpeed
  (params (NewBallSpeed :type Float%20%28double-precision%29))
  (bind _defaultballspeed (Variables|DefaultValues|GetDefaultBallSpeed))
  (bind _maxmodifierfromdefaultvalue (Variables|Static|GetMaxModifierFromDefaultValue))
  (bind _output_get (Variables|Default|SetCurrentBallSpeed (Math|Float|Clamp(Float) NewBallSpeed (/ _defaultballspeed _maxmodifierfromdefaultvalue) (* _defaultballspeed _maxmodifierfromdefaultvalue))))
  (Default|CallOnBallVelocityChanged _output_get))

(fn GetCartWidth
  (return (Variables|Default|GetCurrentCartWidth)))

(fn GetBallSpeed
  (return (Variables|Default|GetCurrentBallSpeed)))

(fn GetBallSize
  (return (Variables|Default|GetCurrentBallSize)))

(fn SpawnBall
  (params (SpawnTransform :type Transform) (Owner :type Actor%20Object%20Reference) (VelocityVector :type Vector))
  (if (Ball|IsAllowSpawnBall)
    (bind _spawnedball (Ball|SpawnBallInternal SpawnTransform Owner VelocityVector))
    (bind _result (Math|Integer|DecrementInt (Variables|Default|GetBallsRemaining))
      (:%20%20
        (Default|CallOnBallsRemainingChanged _result)
        (return _spawnedball true)))
    (else
      (return 0 false))))

(fn DestroyBall
  (params (Item :type BP%20Ball%20Object%20Reference%20%28by%20ref%29))
  (Utilities|Array|RemoveItem (Variables|Default|GetBalls) Item)
  (if (Utilities|Array|IsEmpty (Variables|Default|GetBalls))
    (if (Ball|IsAllowSpawnBall)
      (Default|CallOnSpawnBall)
      (else
        (CallFunction|GameOverInternal)))))

(fn OnDestroyBlock
  (params (Block :type BP%20Block%20Object%20Reference))
  (Utilities|FlowControl|Sequence
    (:then_0
      ;[0.2708 0.2708 0.2708 1 40] Score
      (bind _output_get (Variables|Default|SetScore (+ (* (- (Variables|/Game/Root/GameFramework/GameObjects/Blocks/BP_Block.BP_Block_C|GetMaxHP Block) 1) (Variables|/Script/Arkanoid.ArkanoidGameSettingsAsset|GetBlockPerHPScoreModifier (Variables|Default|GetSettingsAsset))) (Variables|/Script/Arkanoid.ArkanoidGameSettingsAsset|GetBlockScore (Variables|Default|GetSettingsAsset)) (Variables|Default|GetScore))))
      (Default|CallOnScoreUpdated _output_get))
    (:then_1
      (PowerUp|SpawnPowerUp (Transformation|GetActorLocation Block)))))

(fn GetBlockHeight
  (return (Variables|/Script/Arkanoid.ArkanoidGameSettingsAsset|GetDefaultBlockHeight (Variables|Default|GetSettingsAsset))))

(fn GetBlockWidth
  (return (Variables|/Script/Arkanoid.ArkanoidGameSettingsAsset|GetDefaultBlockWidth (Variables|Default|GetSettingsAsset))))

(fn GetColorPerBlockHP
  (params (HP :type Integer))
  (if (Utilities|Array|IsValidIndex (Variables|/Script/Arkanoid.ArkanoidGameSettingsAsset|GetColorPerHP (Variables|Default|GetSettingsAsset)) HP)
    (return (Utilities|Array|Get(acopy) (Variables|/Script/Arkanoid.ArkanoidGameSettingsAsset|GetColorPerHP (Variables|Default|GetSettingsAsset)) HP))
    (else
      (return ""))))

(fn GetAreaWidth
  (return (Variables|/Script/Arkanoid.ArkanoidGameSettingsAsset|GetGameAreaWidth (Variables|Default|GetSettingsAsset))))

(fn GetPowerUpFallSpeed
  (return (Variables|/Script/Arkanoid.ArkanoidGameSettingsAsset|GetFallSpeed (Variables|Default|GetSettingsAsset))))

(fn GetPowerUpSize
  (return (Variables|/Script/Arkanoid.ArkanoidGameSettingsAsset|GetPowerUpSize (Variables|Default|GetSettingsAsset))))

(fn TripleBallPowerUp
  (bind _output_get (LocalVariables|SetCachedBalls (Variables|Default|GetBalls)))
  (Utilities|FlowControl|Sequence
    (:then_0
      _)
    (:then_1
      _))
  (bind _unitvector (CallFunction|GetRandomUnitVector2D (.OutItem (Utilities|Array|Random _output_get))))
  (bind (_spawnedball _bspawned) (Ball|SpawnBallInternal (Math|Transform|MakeTransform (+ (Transformation|GetActorLocation (.OutItem (Utilities|Array|Random _output_get))) (* _unitvector (* (Variables|Default|GetCurrentBallSize) 2.0)))) 0 _unitvector))
  (if _bspawned
    (Default|Activate _spawnedball)))

(fn GetRandomUnitVector2D
  (params (From :type Actor%20Object%20Reference))
  (return (Math|Vector|Normalize (Math|Vector|Lerp(Vector) (* (Math|Float|SelectFloat 1.0 -1.0 (Math|Random|RandomBool)) (Transformation|GetActorUpVector From)) (* (Transformation|GetActorForwardVector From) (Math|Float|SelectFloat 1.0 -1.0 (Math|Random|RandomBool))) (Math|Random|RandomFloat)))))

(fn SpawnBallInternal
  (params (SpawnTransform :type Transform) (Owner :type Actor%20Object%20Reference) (VelocityVector :type Vector))
  (bind _returnvalue (Game|SpawnActorfromClass "/Game/Root/GameFramework/GameObjects/Ball/BP_Ball.BP_Ball_C" SpawnTransform "AlwaysSpawn" "MultiplyWithRoot" Owner VelocityVector 0))
  (Utilities|Array|Add (Variables|Default|GetBalls) _returnvalue)
  (return _returnvalue true))

(fn SpawnPowerUp
  (params (Location :type Vector))
  (for _array_element (Variables|/Script/Arkanoid.ArkanoidGameSettingsAsset|GetPowerUpData (Variables|Default|GetSettingsAsset))
    (if (>= (.Chance (Utilities|Struct|BreakPowerUpData _array_element)) (Math|Random|RandomFloat))
      (Game|SpawnActorfromClass (.PowerUpClass (Utilities|Struct|BreakPowerUpData _array_element)) (Math|Transform|MakeTransform Location) "Undefined" "MultiplyWithRoot" 0 0)
      (return)))
  (return))

(fn IncreaseBallSize
  (Game|SetBallSize (+ (Variables|Default|GetCurrentBallSize) (* (Variables|Static|GetModifierFromDefaultValue) (Variables|DefaultValues|GetDefaultBallSize)))))

(fn DecreaseBallSize
  (Game|SetBallSize (- (Variables|Default|GetCurrentBallSize) (* (Variables|Static|GetModifierFromDefaultValue) (Variables|DefaultValues|GetDefaultBallSize)))))

(fn IncreaseBallSpeed
  (Game|SetBallSpeed (+ (Variables|Default|GetCurrentBallSpeed) (* (Variables|Static|GetModifierFromDefaultValue) (Variables|DefaultValues|GetDefaultBallSpeed)))))

(fn DecreaseBallSpeed
  (Game|SetBallSpeed (- (Variables|Default|GetCurrentBallSpeed) (* (Variables|Static|GetModifierFromDefaultValue) (Variables|DefaultValues|GetDefaultBallSpeed)))))

(fn LifeUp
  (bind _result (Math|Integer|IncrementInt (Variables|Default|GetBallsRemaining))
    (:%20%20
      (Default|CallOnBallsRemainingChanged _result))))

(fn GetBallsRemaining
  (return (Variables|Default|GetBallsRemaining)))

(fn IncreaseCartWidth
  (Game|SetCartWidth (+ (Variables|Default|GetCurrentCartWidth) (* (Variables|Static|GetModifierFromDefaultValue) (Variables|DefaultValues|GetDefaultCartWidth)))))

(fn DecreaseCartWidth
  (Game|SetCartWidth (- (Variables|Default|GetCurrentCartWidth) (* (Variables|Static|GetModifierFromDefaultValue) (Variables|DefaultValues|GetDefaultCartWidth)))))

(fn GetCurrentLevel
  (return (Variables|Default|GetCurrentLevel)))

(fn GetLevelData
  (return (Utilities|Array|Get(acopy) (Variables|/Script/Arkanoid.ArkanoidGameSettingsAsset|GetLevels (Variables|Default|GetSettingsAsset)) (Variables|Default|GetCurrentLevel))))

(fn FinishLevel
  (if (Utilities|Array|IsValidIndex (Variables|/Script/Arkanoid.ArkanoidGameSettingsAsset|GetLevels (Variables|Default|GetSettingsAsset)) (+ (Variables|Default|GetCurrentLevel) 1))
    (Default|CallOnFinishLevel)
    (else
      (CallFunction|GameEndInternal))))

(fn StartNewLevel
  (bind _result (Math|Integer|IncrementInt (Variables|Default|GetCurrentLevel))
    (:%20%20
      (if (Utilities|Array|IsValidIndex (Variables|/Script/Arkanoid.ArkanoidGameSettingsAsset|GetLevels (Variables|Default|GetSettingsAsset)) _result)
        (Default|CallOnStartNewLevel (Variables|Default|GetCurrentLevel))
        (else
          (CallFunction|GameEndInternal))))))

(fn GameEndInternal
  (Variables|Default|SetbGameEnd true)
  (Default|CallOnGameEnd))

(fn GameOverInternal
  (if (not (Variables|Default|GetbGameEnd))
    (Default|CallOnGameOver)))

(fn Pause
  (Game|SetGamePaused true))

(fn UnPause
  (Game|SetGamePaused false))