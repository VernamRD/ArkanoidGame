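; Base Blueprint for falling power-ups that trigger an overridable pickup effect when collected.
; On BeginPlay it reads size and fall speed from BP_GameState, then builds an icon-textured quad with Geometry Script on a dynamic mesh and sizes the overlap box to match.
; Tick moves it down along Z without sweep.
; A box overlap with an actor that has a valid owner calls the empty OnPickuped hook, then destroys the power-up.
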(event OnComponentBeginOverlap(Box)
  (params (OverlappedComponent :type Primitive%20Component%20Object%20Reference) (OtherActor :type Actor%20Object%20Reference) (OtherComp :type Primitive%20Component%20Object%20Reference) (OtherBodyIndex :type Integer) (bFromSweep :type Boolean) (SweepResult :type Hit%20Result%20Structure%20%28by%20ref%29))
  (Utilities|IsValid (Components|GetOwner OtherActor)
    (:Is%20Valid
      (CallFunction|OnPickuped (Variables|Default|GetGameState))
      (Actor|DestroyActor))))

(event EventBeginPlay
  (bind _asbp_game_state (Utilities|Casting|CastToBP_GameState (Game|GetGameState)))
  (bind _output_get (Variables|Default|SetGameState _asbp_game_state))
  (Utilities|FlowControl|Sequence
    (:then_0
      (CallFunction|SetupPowerUp (Default|GetPowerUpSize _output_get)))
    (:then_1
      (Variables|Default|SetFall%20Speed (Default|GetPowerUpFallSpeed _output_get)))))

(event Collision|EventActorBeginOverlap
  (params (OtherActor :type Actor%20Object%20Reference)))

(event EventTick
  (params (DeltaSeconds :type Float%20%28single-precision%29))
  (Transformation|AddActorWorldOffset (Math|Vector|MakeVectorNetQuantize 0.0 0.0 (* (* DeltaSeconds (Variables|Default|GetFall%20Speed)) -1.0))))

(fn ConstructionScript)

(fn SetupPowerUp
  (params (PowerUpSize :type Float%20%28single-precision%29))
  (bind _returnvalue (/ PowerUpSize 2.0))
  (bind _returnvalue_2 (DynamicMeshComponent|GetDynamicMesh (Variables|Default|GetDynamicMesh)))
  (bind _returnvalue_3 (DynamicMesh|Reset _returnvalue_2))
  (GeometryScript|Scene|SetComponentMaterialList (Variables|Default|GetDynamicMesh) (Utilities|Array|MakeArray (Variables|Default|GetIcon)) 0)
  (Class|GeometryScriptLibraryMeshPrimitiveFunctions|AppendRectangleXY :TargetMesh _returnvalue_3 :Transform (Math|Transform|MakeTransform "0, 0, 0" "180.000000,0.000000,180.000000") :DimensionX PowerUpSize :DimensionY PowerUpSize :StepsWidth 1 :StepsHeight 1 :Debug 0)
  (Components|Box|SetBoxExtent (Variables|Default|GetBox) (Math|Vector|MakeVector _returnvalue _returnvalue 1e+02) true))

(fn OnPickuped
  (params (GameState :type BP%20Game%20State%20Object%20Reference)))